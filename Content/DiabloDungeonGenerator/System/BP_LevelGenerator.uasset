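; Level generator actor that builds a random tile-based dungeon on BeginPlay.
; GenerateTileLayout random-walks a grid from the start tile (first step south) through generic tiles to an end tile, recording cardinal connections in a map.
; SpawnTileLayout spawns a random tile class whose default connections match each generic or end cell, attaching every tile to the generator.
; The generator then rotates 45 degrees, turning the whole layout.
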(event EventBeginPlay
  (Generation|GenerateTileLayout)
  (Generation|SpawnTileLayout)
  (Transformation|SetActorRotation "0,45.000000, 0"))

(event Collision|EventActorBeginOverlap
  (params (OtherActor :type Actor%20Object%20Reference)))

(event EventTick
  (params (DeltaSeconds :type Float%20%28single-precision%29)))

(fn ConstructionScript)

(fn SpawnTile
  (params (TileToSpawn :type BP%20Tile%20Class%20Reference) (SpawnTransform :type Transform))
  (bind _returnvalue (Game|SpawnActorfromClass TileToSpawn SpawnTransform "Undefined" 0 0))
  (Transformation|AttachActorToActor _returnvalue self "None" "KeepRelative" "SnapToTarget" "KeepRelative" true))

(fn GenerateTileLayout
  (Utilities|Map|Add :TargetMap (Variables|Default|GetTileLayout) :Value (Utilities|Struct|MakeStruct_TileInformation "NewEnumerator1" (LocalVariables|GetEmptyConnection)))
  (for _index (range 1 (Variables|Default|GetValueAmount))
    (bind (_foundlocation _todirection) (CallFunction|FindRandomNextLocation (LocalVariables|GetpreviousLocation) (select (== (Utilities|Map|Length (Variables|Default|GetTileLayout)) 1) "NewEnumerator1" "NewEnumerator4")))
    (LocalVariables|SetfoundLocation _foundlocation)
    (LocalVariables|Setcoming%20FromCardinal _todirection)
    (Utilities|Map|Add (Variables|Default|GetTileLayout) (LocalVariables|GetfoundLocation) (Utilities|Struct|MakeStruct_TileInformation "NewEnumerator0" (LocalVariables|GetEmptyConnection)))
    (CallFunction|ConnectTiles (LocalVariables|GetpreviousLocation) (LocalVariables|GetfoundLocation) (LocalVariables|Getcoming%20FromCardinal))
    (LocalVariables|SetpreviousLocation (LocalVariables|GetfoundLocation)))
  (bind (_foundlocation_2 _todirection_2) (CallFunction|FindRandomNextLocation (LocalVariables|GetpreviousLocation) "NewEnumerator4"))
  (Utilities|Map|Add (Variables|Default|GetTileLayout) _foundlocation_2 (Utilities|Struct|MakeStruct_TileInformation "NewEnumerator2" (LocalVariables|GetEmptyConnection)))
  (CallFunction|ConnectTiles (LocalVariables|GetpreviousLocation) _foundlocation_2 _todirection_2))

(fn SpawnTileLayout
  (bind _tilelayout (Variables|Default|GetTileLayout))
  (bind _keys (Utilities|Map|Keys _tilelayout))
  (for _array_element _keys
    (Generation|SpawnTile (CallFunction|GetTIleClass (.type (.Value (Utilities|Map|Find _tilelayout _array_element))) (.directions (.Value (Utilities|Map|Find _tilelayout _array_element)))) (CallFunction|GetTIleLocation _array_element))))

(fn GetTIleClass
  (params (TileType :type Enum_TileType%20Enum :default "NewEnumerator0") (ToDirection :type Map%20of%20Enum_CardinalPoint%20Enums%20to%20Booleans :default "NewEnumerator0"))
  (if (Utilities|Enum|Equal(Enum) TileType "NewEnumerator1")
    (return "/Game/DiabloDungeonGenerator/Tiles/BP_StartTile.BP_StartTile_C")
    (elif (Utilities|Enum|Equal(Enum) TileType "NewEnumerator0")
      (bind _output (CallFunction|FindRandomValidTile (Variables|Default|GetGenericTileList) ToDirection))
      (return _output)
      (elif (Utilities|Enum|Equal(Enum) TileType "NewEnumerator2")
        (bind _output_2 (CallFunction|FindRandomValidTile (Variables|Default|GetEndTileList_0) ToDirection))
        (return _output_2)
        (else
          (return "/Game/DiabloDungeonGenerator/Tiles/BP_StartTile.BP_StartTile_C"))))))

(fn GetTIleLocation
  (params (inTileLocation :type Vector%202D%20Structure))
  (bind _tilesize (Variables|Default|GetTileSize))
  (return (Math|Transform|MakeTransform (Math|Vector|MakeVector (* (.x inTileLocation) (.x _tilesize)) (* (.y inTileLocation) (.y _tilesize)) 0.0) "0, 0, 0" "1.000000,1.000000,1.000000")))

(fn FindRandomNextLocation
  (params (StartingLocation :type Vector%202D%20Structure) (Wanted%20Direction :type Enum_CardinalPoint%20Enum :default "NewEnumerator0"))
  (bind _locationstoseeknew (LocalVariables|GetLocationsToSeekNew))
  (if (Utilities|Enum|Equal(Enum) Wanted%20Direction "NewEnumerator4")
    (bind _keys (Utilities|Map|Keys (LocalVariables|GetLocationsToSeekNew)))
    (for _array_element _keys
      (if (CallFunction|IsTileUsed (+ StartingLocation (.Value (Utilities|Map|Find (LocalVariables|GetLocationsToSeekNew) _array_element))))
        (Utilities|Map|Remove (LocalVariables|GetLocationsToSeekNew) _array_element)))
    (bind _keys_2 (Utilities|Map|Keys _locationstoseeknew))
    (bind _output_get (LocalVariables|SetrandomizedResult (Utilities|Array|Get(acopy) _keys_2 (Math|Random|RandomIntegerinRange 0 (Utilities|Array|LastIndex _keys_2)))))
    (return (+ (.Value (Utilities|Map|Find _locationstoseeknew _output_get)) StartingLocation) (LocalVariables|GetrandomizedResult))
    (else
      (return (.Value (Utilities|Map|Find (LocalVariables|GetLocationsToSeekNew) Wanted%20Direction)) Wanted%20Direction))))

(fn IsTileUsed
  (params (AtLocation :type Vector%202D%20Structure))
  (return (.ReturnValue (Utilities|Map|Find (Variables|Default|GetTileLayout) AtLocation))))

(fn ConnectTiles
  (params (Tile%20One :type Vector%202D%20Structure) (Tile%20Two :type Vector%202D%20Structure) (From%20Cardnal :type Enum_CardinalPoint%20Enum :default "NewEnumerator0"))
  (CallFunction|SetConnection Tile%20One From%20Cardnal true)
  (CallFunction|SetConnection Tile%20Two (CallFunction|ReverseCardinal From%20Cardnal) true))

(fn SetConnection
  (params (Tile :type Vector%202D%20Structure) (ToCardnalPoint :type Enum_CardinalPoint%20Enum :default "NewEnumerator0") (Enabled :type Boolean))
  (bind _tilelayout (Variables|Default|GetTileLayout))
  (bind (_value _returnvalue) (Utilities|Map|Find _tilelayout Tile))
  (if _returnvalue
    (LocalVariables|SettempDirection (.directions _value))
    (Utilities|Map|Add (LocalVariables|GettempDirection) ToCardnalPoint Enabled)
    (Utilities|Map|Add (Variables|Default|GetTileLayout) Tile (Utilities|Struct|MakeStruct_TileInformation (.type _value) (LocalVariables|GettempDirection)))))

(fn ReverseCardinal
  (params (InCardnal :type Enum_CardinalPoint%20Enum :default "NewEnumerator0"))
  (return (Utilities|Select :Index InCardnal :NewEnumerator0 "NewEnumerator1" :NewEnumerator1 "NewEnumerator0" :NewEnumerator2 "NewEnumerator3" :NewEnumerator3 "NewEnumerator2" :NewEnumerator4 "NewEnumerator0")))

(fn AreConnectionMatching?
  (params (In%20Connection :type Map%20of%20Enum_CardinalPoint%20Enums%20to%20Booleans :default "NewEnumerator0") (Against%20Connection :type Map%20of%20Enum_CardinalPoint%20Enums%20to%20Booleans :default "NewEnumerator0"))
  (LocalVariables|SetbTempValidTile true)
  (bind _keys (Utilities|Map|Keys In%20Connection))
  (bind _array_element (Utilities|Array|ForEachLoopwithBreak _keys :!label _label)
    (:LoopBody
      (if (!= (.Value (Utilities|Map|Find Against%20Connection _array_element)) (.Value (Utilities|Map|Find In%20Connection _array_element)))
        (LocalVariables|SetbTempValidTile false)
        (goto _label Break)))
    (:Completed
      (return (LocalVariables|GetbTempValidTile)))))

(fn FindRandomValidTile
  (params (Array :type Array%20of%20BP%20Tile%20Class%20References) (In%20Connection :type Map%20of%20Enum_CardinalPoint%20Enums%20to%20Booleans :default "NewEnumerator0"))
  (bind _validtiles (LocalVariables|GetvalidTiles))
  (for _array_element Array
    (if (CallFunction|AreConnectionMatching? In%20Connection (Utilities|GetClassDefaults _array_element))
      (Utilities|Array|Add (LocalVariables|GetvalidTiles) _array_element)))
  (return (Utilities|Array|Get(acopy) _validtiles (Math|Random|RandomIntegerinRange 0 (Utilities|Array|LastIndex _validtiles)))))