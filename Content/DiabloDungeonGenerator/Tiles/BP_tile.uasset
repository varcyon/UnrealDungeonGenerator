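; Dungeon tile actor for the Diablo-style generator, shaping its openings from the TileConnection map of directions to booleans.
; On BeginPlay, GenerateConnectors destroys the wall on each connected side and the connector on each unconnected side, revealing direction markers for connected sides.
; BeginPlay then assigns the floor a flat color material based on TileType.
; The construction script also reveals those markers, without removing any components.
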(event EventBeginPlay
  (CallFunction|GenerateConnectors)
  (if (Utilities|Enum|Equal(Enum) (Variables|Metrics|GetTileType) "NewEnumerator3")
    (Rendering|Material|SetMaterial (Variables|Default|GetFloor) 0 "/Engine/BasicShapes/FlatRed.FlatRed")
    (elif (Utilities|Enum|Equal(Enum) (Variables|Metrics|GetTileType) "NewEnumerator1")
      (Rendering|Material|SetMaterial (Variables|Default|GetFloor) 0 "/Engine/BasicShapes/FlatGreen.FlatGreen")
      (elif (Utilities|Enum|Equal(Enum) (Variables|Metrics|GetTileType) "NewEnumerator0")
        (Rendering|Material|SetMaterial (Variables|Default|GetFloor) 0 "/Engine/BasicShapes/FlatWhite.FlatWhite")
        (elif (Utilities|Enum|Equal(Enum) (Variables|Metrics|GetTileType) "NewEnumerator4")
          (Rendering|Material|SetMaterial (Variables|Default|GetFloor) 0 "/Engine/BasicShapes/FlatOrange.FlatOrange")
          (elif (Utilities|Enum|Equal(Enum) (Variables|Metrics|GetTileType) "NewEnumerator2")
            (Rendering|Material|SetMaterial (Variables|Default|GetFloor) 0 "/Engine/BasicShapes/FlatBlue.FlatBlue")))))))

(event Collision|EventActorBeginOverlap
  (params (OtherActor :type Actor%20Object%20Reference)))

(event EventTick
  (params (DeltaSeconds :type Float%20%28single-precision%29)))

(fn ConstructionScript
  (bind _tileconnection (Variables|Metrics|GetTileConnection))
  (bind _keys (Utilities|Map|Keys _tileconnection))
  (for _array_element _keys
    (if (.Value (Utilities|Map|Find _tileconnection _array_element))
      (Rendering|SetVisibility (Utilities|Select :Index _array_element :NewEnumerator0 (Variables|Default|GetNorthDirection) :NewEnumerator1 (Variables|Default|GetSouthDirection) :NewEnumerator2 (Variables|Default|GetEastDirection) :NewEnumerator3 (Variables|Default|GetWestDirection) :NewEnumerator4 0) (.Value (Utilities|Map|Find _tileconnection _array_element)) false)
      (Development|SetHiddeninGame (Utilities|Select :Index _array_element :NewEnumerator0 (Variables|Default|GetNorthDirection) :NewEnumerator1 (Variables|Default|GetSouthDirection) :NewEnumerator2 (Variables|Default|GetEastDirection) :NewEnumerator3 (Variables|Default|GetWestDirection) :NewEnumerator4 0) (not (.Value (Utilities|Map|Find _tileconnection _array_element))) false))))

(fn GenerateConnectors
  (bind _tileconnection (Variables|Metrics|GetTileConnection))
  (bind _keys (Utilities|Map|Keys _tileconnection))
  (for _array_element _keys
    (if (.Value (Utilities|Map|Find _tileconnection _array_element))
      (Rendering|SetVisibility (Utilities|Select :Index _array_element :NewEnumerator0 (Variables|Default|GetNorthDirection) :NewEnumerator1 (Variables|Default|GetSouthDirection) :NewEnumerator2 (Variables|Default|GetEastDirection) :NewEnumerator3 (Variables|Default|GetWestDirection) :NewEnumerator4 0) (.Value (Utilities|Map|Find _tileconnection _array_element)) false)
      (Development|SetHiddeninGame (Utilities|Select :Index _array_element :NewEnumerator0 (Variables|Default|GetNorthDirection) :NewEnumerator1 (Variables|Default|GetSouthDirection) :NewEnumerator2 (Variables|Default|GetEastDirection) :NewEnumerator3 (Variables|Default|GetWestDirection) :NewEnumerator4 0) (not (.Value (Utilities|Map|Find _tileconnection _array_element))) false)
      (Components|DestroyComponent (Utilities|Select :Index _array_element :NewEnumerator0 (Variables|Default|GetNorthernWall) :NewEnumerator1 (Variables|Default|GetSouthernWall) :NewEnumerator2 (Variables|Default|GetEasternWall) :NewEnumerator3 (Variables|Default|GetWesternWall) :NewEnumerator4 0))
      (else
        (Components|DestroyComponent (Utilities|Select :Index _array_element :NewEnumerator0 (Variables|Default|GetNorthernConnector) :NewEnumerator1 (Variables|Default|GetSouthernConnector) :NewEnumerator2 (Variables|Default|GetEasternConnector) :NewEnumerator3 (Variables|Default|GetWesternConnector) :NewEnumerator4 0))))))